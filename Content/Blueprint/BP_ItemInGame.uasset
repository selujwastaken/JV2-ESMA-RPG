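; BP_ItemInGame is a world item actor that displays an item's mesh and name.
; On BeginPlay it sets its static mesh and text label from the CurrentItem data.
; Every tick it rotates the name label to face the top-down controller's camera, keeping it readable from the player's view.
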(event `self.ReceiveTick`
  (params (DeltaSeconds :type "Float (single-precision)"))
  (bind _name (`self.Name`))
  (`SceneComponent.K2_SetWorldRotation` _name (`KismetMathLibrary.FindLookAtRotation` (`SceneComponent.K2_GetComponentLocation` _name) (`PlayerCameraManager.GetCameraLocation` (`PlayerController.PlayerCameraManager` (`/Game/Blueprint/BP_FL_Shortcut.GetTopDownControler`)))) false false))

(event `self.ReceiveBeginPlay`
  (`StaticMeshComponent.SetStaticMesh` (`self.StaticMesh`) (`/Game/Blueprint/Data/Data_Asset/BP_DA_Items.MeshDisplay` (`self.CurrentItem`)))
  (`TextRenderComponent.K2_SetText` (`self.Name`) (`/Game/Blueprint/Data/Data_Asset/BP_DA_Items.Name` (`self.CurrentItem`))))

(fn `UserConstructionScript`)