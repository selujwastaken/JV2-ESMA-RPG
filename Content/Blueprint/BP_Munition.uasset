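; BP_Munition is a fireable projectile actor that destroys itself on impact or after a timeout.
; FireMunition spawns a Niagara effect attached to the Scene component, sets IsFired, activates the projectile movement, and destroys the actor after a short delay.
; A hit on the Trigger component checks IsFired, prints a debug "BOOM" and jumps to the same destroy step.
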(event `FireMunition`
  (bind _scene (`self.Scene`))
  (`NiagaraFunctionLibrary.SpawnSystemAttached` "/Game/Blueprint/NewNiagaraSystem.NewNiagaraSystem" _scene "None" (`SceneComponent.RelativeLocation` _scene) (struct) "SnapToTarget")
  (set `self.IsFired` true)
  (`ActorComponent.Activate` (`self.ProjectileMovement`) false)
  (`KismetSystemLibrary.Delay` 5.0)
  (`self.K2_DestroyActor` :!label _label))

(event `self.Trigger.OnComponentHit`
  (params (HitComponent :type "PrimitiveComponent Object Reference") (OtherActor :type "Actor Object Reference") (OtherComp :type "PrimitiveComponent Object Reference") (NormalImpulse :type "Vector Structure") (Hit :type "HitResult Structure (by ref)"))
  (`self.IsFired`
    (:`then`
      (`KismetSystemLibrary.PrintString` "BOOM")
      (goto _label))
    (:`else`)))

(fn `UserConstructionScript`)