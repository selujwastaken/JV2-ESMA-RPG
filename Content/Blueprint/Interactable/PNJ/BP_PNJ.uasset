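; BP_PNJ is an interactable NPC that toggles a dialogue mode with the player each time Interact fires.
; A FlipFlop alternates entering and leaving: entry snaps the player to the Arrow transform, shows Description, switches the view to the NPC and blocks movement.
; Exit hides Description, returns the view to the pawn and restores movement.
; Both branches set InDialogue on the player's ABP_Player anim instance.
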(event `self.Interact`
  (bind _top_down_player_controler_ (`/Game/Blueprint/BP_FL_Shortcut.GetTopDownControler`))
  (bind _top_down_player_controler__2 (`/Game/Blueprint/BP_FL_Shortcut.GetTopDownControler`))
  (`/Engine/EditorBlueprintResources/StandardMacros.FlipFlop`
    (:`A`
      (bind _asbp_top_down_character (cast `/Game/Blueprint/BP_TopDownCharacter` (`GameplayStatics.GetPlayerPawn` 0)))
      (bind _asabp_player (cast `/Game/Characters/Mannequins/Anims/ABP_Player` (`SkeletalMeshComponent.GetAnimInstance` (`Character.Mesh` _asbp_top_down_character))))
      (set `/Game/Characters/Mannequins/Anims/ABP_Player.InDialogue` true _asabp_player)
      (`self.K2_SetActorTransform` _asbp_top_down_character (`SceneComponent.K2_GetComponentToWorld` (`self.Arrow`)) false false)
      (`SceneComponent.SetVisibility` (`self.Description`) true false)
      (`PlayerController.SetViewTargetWithBlend` _top_down_player_controler__2 self 0.0 "VTBlend_Linear" 0.0 false)
      (set `/Game/Blueprint/BP_TopDownController.Can Move` false _top_down_player_controler__2))
    (:`B`
      (bind _asbp_top_down_character_2 (cast `/Game/Blueprint/BP_TopDownCharacter` (`GameplayStatics.GetPlayerPawn` 0)))
      (bind _asabp_player_2 (cast `/Game/Characters/Mannequins/Anims/ABP_Player` (`SkeletalMeshComponent.GetAnimInstance` (`Character.Mesh` _asbp_top_down_character_2))))
      (set `/Game/Characters/Mannequins/Anims/ABP_Player.InDialogue` false _asabp_player_2)
      (`SceneComponent.SetVisibility` (`self.Description`) false false)
      (`PlayerController.SetViewTargetWithBlend` _top_down_player_controler_ (`Controller.K2_GetPawn` _top_down_player_controler_) 0.0 "VTBlend_Linear" 0.0 false)
      (set `/Game/Blueprint/BP_TopDownController.Can Move` true _top_down_player_controler_))))

(fn `UserConstructionScript`)